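; Platform actor that rocks its static mesh back and forth around the roll axis.
; BeginPlay caches the mesh's initial relative rotation.
; Each Tick accumulates running time and combines that starting rotation with a sine-driven roll offset, scaled by the Speed and Amplitude variables.
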(event `self.ReceiveBeginPlay`
  (set `self.InitialRotation` (`SceneComponent.RelativeRotation` (`self.StaticMesh`))))

(event `self.ReceiveTick`
  (params (DeltaSeconds :type "Float (single-precision)"))
  (bind _output_get (set `self.RunningTime` (+ (`self.RunningTime`) DeltaSeconds)))
  (`SceneComponent.K2_SetRelativeRotation` (`self.StaticMesh`) (`KismetMathLibrary.ComposeRotators` (`self.InitialRotation`) (`KismetMathLibrary.MakeRotator` (* (`KismetMathLibrary.Sin` (* _output_get (`self.Speed`))) (`self.Amplitude`)))) false false))

(fn `UserConstructionScript`)